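; BPC_Rifle is an automatic rifle that fires projectiles for the third-person character.
; Fire starts a looping timer whose negative start delay makes the first shot immediate; EndFire or empty ammo clears it.
; Each shot spends ammo, spawns a BP_Projectile with controller rumble and Wwise audio, and launches it along the character's ActionValue input in the Y/Z plane, or actor forward without input.
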(event Custom|Shoot
  (bind _as_bp_third_person_character (Variables|Default|GetAs%20BP%20Third%20Person%20Character))
  (bind _ammo (Variables|Default|GetAmmo))
  (bind _action_value (Variables|/Game/ThirdPerson/Blueprints/BP_ThirdPersonCharacter.BP_ThirdPersonCharacter_C|GetAction%20Value _as_bp_third_person_character))
  (bind (_x _y) (Math|Vector2D|BreakVector2D _action_value))
  (if (not (<= _ammo 0))
    (Math|Integer|DecrementInt _ammo
      (:%20%20
        (bind _returnvalue (Game|SpawnActorfromClass "/Game/Blueprint/Projectile/BP_Projectile.BP_Projectile_C" (Transformation|GetWorldTransform (Variables|Default|GetProjectileSpawn)) "Undefined" "MultiplyWithRoot" 0 1e+01 0))
        (Game|Feedback|ClientPlayForceFeedback (Game|GetPlayerController 0) "/Game/FF_Rifle.FF_Rifle" "None" false false false)
        (Variables|/Script/Engine.MovementComponent|SetVelocity (Variables|/Game/Blueprint/Projectile/BP_Projectile.BP_Projectile_C|GetProjectileMovement _returnvalue) (* (select (and (== _x 0.0) (== _y 0.0)) (Transformation|GetActorForwardVector _as_bp_third_person_character) (Math|Vector|Normalize (Math|Vector|MakeVector 0.0 _x _y))) 1.2e+03))
        (Class|AkGameplayStatics|PostEvent "/Game/WwiseAudio/Event/Play_RND_FusilShoot_01.Play_RND_FusilShoot_01")))
    (else
      (Utilities|Time|ClearandInvalidateTimerbyHandle (Variables|Default|GetFireTimer))
      (Class|AkGameplayStatics|PostEvent "/Game/WwiseAudio/Event/Stop_RND_FusilShoot.Stop_RND_FusilShoot"))))

(event EventFire
  (bind _returnvalue (Math|Float|MakeLiteralFloat 0.3))
  (bind _returnvalue_2 (Utilities|Time|SetTimerbyEvent (delegate Custom|Shoot) _returnvalue true (* _returnvalue -1.0)))
  (Variables|Default|SetFireTimer _returnvalue_2))

(event EventEndFire
  (Utilities|Time|ClearandInvalidateTimerbyHandle (Variables|Default|GetFireTimer)))

(event EventBeginPlay)

(fn ConstructionScript
  (|CallParentFunction))