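; BP_GigaChadOneWay is a one-way collision actor that lets the third-person character pass through its static mesh from the side covered by the Down trigger.
; The construction script sets the mesh's initial Pawn response from the StartCollision variable.
; Overlapping Down switches that response to Ignore, and leaving it restores Block.
; A separate OneWay event also sets it to Ignore.
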(event OnComponentBeginOverlap(Down)
  (params (OverlappedComponent :type Primitive%20Component%20Object%20Reference) (OtherActor :type Actor%20Object%20Reference) (OtherComp :type Primitive%20Component%20Object%20Reference) (OtherBodyIndex :type Integer) (bFromSweep :type Boolean) (SweepResult :type Hit%20Result%20Structure%20%28by%20ref%29))
  (Utilities|Casting|CastToBP_ThirdPersonCharacter OtherActor)
  (Collision|SetCollisionResponsetoChannel (Variables|Default|GetStaticMesh) "ECC_Pawn" "ECR_Ignore"))

(event OnComponentEndOverlap(Down)
  (params (OverlappedComponent :type Primitive%20Component%20Object%20Reference) (OtherActor :type Actor%20Object%20Reference) (OtherComp :type Primitive%20Component%20Object%20Reference) (OtherBodyIndex :type Integer))
  (Utilities|Casting|CastToBP_ThirdPersonCharacter OtherActor)
  (Collision|SetCollisionResponsetoChannel (Variables|Default|GetStaticMesh) "ECC_Pawn" "ECR_Block"))

(event EventOneWay
  (Collision|SetCollisionResponsetoChannel (Variables|Default|GetStaticMesh) "ECC_Pawn" "ECR_Ignore"))

(fn ConstructionScript
  (Collision|SetCollisionResponsetoChannel (Variables|Default|GetStaticMesh) "ECC_Pawn" (Variables|Default|GetStartCollision%20?)))