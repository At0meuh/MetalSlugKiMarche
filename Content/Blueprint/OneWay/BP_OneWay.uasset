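; BP_OneWay is a one-way platform that toggles the collision of its Plateforme component for the third-person character.
; Overlapping the Down trigger disables collision unless the character's IsUp flag is set, and leaving it restores collision.
; Entering or leaving the Up trigger enables collision, or disables it if the character's IsDown flag is set.
; Collision changes apply to the whole component rather than per character.
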(event OnComponentBeginOverlap(Down)
  (params (OverlappedComponent :type Primitive%20Component%20Object%20Reference) (OtherActor :type Actor%20Object%20Reference) (OtherComp :type Primitive%20Component%20Object%20Reference) (OtherBodyIndex :type Integer) (bFromSweep :type Boolean) (SweepResult :type Hit%20Result%20Structure%20%28by%20ref%29))
  (bind _asbp_third_person_character (Utilities|Casting|CastToBP_ThirdPersonCharacter OtherActor))
  (if (not (Variables|/Game/ThirdPerson/Blueprints/BP_ThirdPersonCharacter.BP_ThirdPersonCharacter_C|GetIsUp _asbp_third_person_character))
    (Collision|SetCollisionEnabled (Variables|Default|GetPlateforme) "NoCollision")))

(event OnComponentEndOverlap(Down)
  (params (OverlappedComponent :type Primitive%20Component%20Object%20Reference) (OtherActor :type Actor%20Object%20Reference) (OtherComp :type Primitive%20Component%20Object%20Reference) (OtherBodyIndex :type Integer))
  (Utilities|Casting|CastToBP_ThirdPersonCharacter OtherActor)
  (Collision|SetCollisionEnabled (Variables|Default|GetPlateforme) "QueryAndPhysics"))

(event OnComponentBeginOverlap(Up)
  (params (OverlappedComponent :type Primitive%20Component%20Object%20Reference) (OtherActor :type Actor%20Object%20Reference) (OtherComp :type Primitive%20Component%20Object%20Reference) (OtherBodyIndex :type Integer) (bFromSweep :type Boolean) (SweepResult :type Hit%20Result%20Structure%20%28by%20ref%29))
  (bind _asbp_third_person_character (Utilities|Casting|CastToBP_ThirdPersonCharacter OtherActor))
  (Collision|SetCollisionEnabled (Variables|Default|GetPlateforme) "QueryAndPhysics")
  (if (Variables|/Game/ThirdPerson/Blueprints/BP_ThirdPersonCharacter.BP_ThirdPersonCharacter_C|GetIsDown _asbp_third_person_character)
    (Collision|SetCollisionEnabled (Variables|Default|GetPlateforme) "NoCollision")))

(event OnComponentEndOverlap(Up)
  (params (OverlappedComponent :type Primitive%20Component%20Object%20Reference) (OtherActor :type Actor%20Object%20Reference) (OtherComp :type Primitive%20Component%20Object%20Reference) (OtherBodyIndex :type Integer))
  (bind _asbp_third_person_character (Utilities|Casting|CastToBP_ThirdPersonCharacter OtherActor))
  (Collision|SetCollisionEnabled (Variables|Default|GetPlateforme) "NoCollision")
  (if (not (Variables|/Game/ThirdPerson/Blueprints/BP_ThirdPersonCharacter.BP_ThirdPersonCharacter_C|GetIsDown _asbp_third_person_character))
    (Collision|SetCollisionEnabled (Variables|Default|GetPlateforme) "QueryAndPhysics")))

(fn ConstructionScript)