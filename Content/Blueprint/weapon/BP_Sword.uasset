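; Sword weapon that performs a melee attack on the player's third-person character when Fire is called.
; A DoOnce gates attacks until the montage's notify end, while a FlipFlop alternates between two attack montages.
; On notify begin it plays a Wwise whoosh and controller rumble, then runs a stationary sphere trace in front of the player.
; Hit actors take damage only if they implement BPI_FlammeThrower.
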(event EventBeginPlay
  (|CallParentFunction) ; This node is disabled and will not be called.\nDrag off pins to build functionality.
)

(event Collision|EventActorBeginOverlap
  (params (OtherActor :type Actor%20Object%20Reference)))

(event EventTick
  (params (DeltaSeconds :type Float%20%28single-precision%29)))

(event EventFire
  (bind _returnvalue (Game|GetPlayerCharacter 0))
  (bind _asbp_third_person_character (Utilities|Casting|CastToBP_ThirdPersonCharacter _returnvalue))
  (bind _returnvalue_2 (Transformation|GetActorLocation _asbp_third_person_character))
  (bind _returnvalue_3 (Transformation|GetActorForwardVector _asbp_third_person_character))
  (bind _returnvalue_4 (* _returnvalue_3 1.5e+02))
  (bind _returnvalue_5 (+ _returnvalue_2 _returnvalue_4))
  (Utilities|FlowControl|DoOnce false :!label _label
    (:Completed
      (bind _isa (Utilities|FlowControl|FlipFlop)
        (:A
          _)
        (:B
          _))
      (Animation|Montage|PlayMontage (Variables|/Script/Engine.Character|GetMesh _asbp_third_person_character) (select _isa "/Game/AnimAttackRoot_Montage.AnimAttackRoot_Montage" "/Game/AnimAttackRoot1_Montage.AnimAttackRoot1_Montage") 1.5
        (:OnNotifyBegin
          (Class|AkGameplayStatics|PostEvent "/Game/WwiseAudio/Event/Play_RND_SwordWhoosh.Play_RND_SwordWhoosh" self)
          (Game|Feedback|ClientPlayForceFeedback (Game|GetPlayerController 0) "/Game/FF_Sword.FF_Sword" "None" false false false)
          (bind (_outhit _returnvalue_6) (Collision|SphereTraceByChannel _returnvalue_5 _returnvalue_5 1.2e+02 "TraceTypeQuery1" false 0 "None"))
          (if _returnvalue_6
            (if (Utilities|DoesObjectImplementInterface (.HitActor (Collision|BreakHitResult _outhit)) "/Game/Blueprint/weapon/BPI_FlammeThrower.BPI_FlammeThrower_C")
              (Game|Damage|ApplyDamage (.HitActor (Collision|BreakHitResult _outhit)) 2e+01 0 0))))
        (:OnNotifyEnd
          (goto _label Reset))))))

(fn ConstructionScript
  (|CallParentFunction))