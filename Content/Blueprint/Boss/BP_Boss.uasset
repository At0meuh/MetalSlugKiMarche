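; Boss character that takes damage and ends the game in a win when killed.
; AnyDamage, gated by Dead and CanBeDammaged, lowers HP, plays a hit montage only when InFloor, and flashes a dynamic overlay material through a Timeline.
; At zero HP, a death montage notify shows WBP_EndGame, saves score and time under a hardcoded name, then pauses the game.
; Tick prints HP on screen.
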(event Custom|AnnyDammage
  (bind _alpha (Timeline|Timeline PlayFromStart)
    (:Update
      (Rendering|Material|SetScalarParameterValue (Variables|Default|GetTakeDammage) "opacity" _alpha :!class /Script/Engine.MaterialInstanceDynamic))))

(event EventBeginPlay
  (bind _returnvalue (Rendering|Material|CreateDynamicMaterialInstance "/Game/Material/MI_BossTakesDammage.MI_BossTakesDammage" "None" "None" :!class /Script/Engine.KismetMaterialLibrary))
  (bind _output_get (Variables|Default|SetTakeDammage _returnvalue))
  (Rendering|Material|SetOverlayMaterial (Variables|Character|GetMesh) _output_get :!class /Script/Engine.MeshComponent))

(event EventTick
  (params (DeltaSeconds :type Float%20%28single-precision%29))
  (Development|PrintString (Utilities|String|ToString(Float) (Variables|Default|GetHP)) true true "(R=1.000000,G=0.032916,B=0.000000,A=1.000000)" 0.0))

(event Game|Damage|EventAnyDamage
  (params (Damage :type Float%20%28single-precision%29) (DamageType :type Damage%20Type%20Object%20Reference) (InstigatedBy :type Controller%20Object%20Reference) (DamageCauser :type Actor%20Object%20Reference))
  (bind _returnvalue (Game|GetPlayerCharacter 0))
  (bind _asbp_third_person_character (Utilities|Casting|CastToBP_ThirdPersonCharacter _returnvalue))
  (bind _score (Variables|/Game/ThirdPerson/Blueprints/BP_ThirdPersonCharacter.BP_ThirdPersonCharacter_C|GetScore _asbp_third_person_character))
  (bind _timer (Variables|/Game/ThirdPerson/Blueprints/BP_ThirdPersonCharacter.BP_ThirdPersonCharacter_C|GetTimer _asbp_third_person_character))
  (if (not (Variables|Default|GetDead?))
    (if (Variables|Default|GetCanBeDammaged)
      (if (Variables|Default|GetInFloor?)
        (Animation|Montage|PlayMontage (Variables|Character|GetMesh) "/Game/AnimMageattacked_Montage.AnimMageattacked_Montage"
          (:then
            _)))
      (CallFunction|AnnyDammage)
      (Variables|Default|SetHP (- (Variables|Default|GetHP) Damage))
      (if (<= (Variables|Default|GetHP) 0.0)
        (Variables|Default|SetDead? true)
        (Animation|Montage|PlayMontage (Variables|Character|GetMesh) "/Game/AnimMagedead_Montage.AnimMagedead_Montage"
          (:OnNotifyBegin
            (bind _returnvalue_2 (UserInterface|CreateWidget "/Game/Widget/WBP_EndGame.WBP_EndGame_C" 0 _asbp_third_person_character))
            (UserInterface|Viewport|AddtoViewport _returnvalue_2 0)
            (Default|HandleEndGame _returnvalue_2 true _score _timer)
            (Default|Sauvegarde (.AsBp%20Custom%20Game%20Instance (Utilities|Casting|CastToBp_CustomGameInstance (Game|GetGameInstance))) (Utilities|Struct|MakeST_Score "Nest0r" _score _timer))
            (Game|SetGamePaused true)))))))

(fn ConstructionScript)