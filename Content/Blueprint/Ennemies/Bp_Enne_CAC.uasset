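; Melee enemy Blueprint that extends a parent enemy class by overriding its Attack event.
; After calling the parent, it alternates between two attack montages with a FlipFlop.
; On the montage's notify, a sphere trace with debug drawing checks just in front of the enemy on the Camera channel and applies Damage if it hits BP_ThirdPersonCharacter.
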(event EventBeginPlay)

(event Collision|EventActorBeginOverlap
  (params (OtherActor :type Actor%20Object%20Reference)))

(event EventTick
  (params (DeltaSeconds :type Float%20%28single-precision%29))
  (|CallParentFunction DeltaSeconds) ; This node is disabled and will not be called.\nDrag off pins to build functionality.
)

(event EventAttack
  (bind _returnvalue (Transformation|GetActorLocation))
  (bind _returnvalue_2 (Transformation|GetActorForwardVector))
  (bind _returnvalue_3 (* _returnvalue_2 1.5e+02))
  (bind _returnvalue_4 (+ _returnvalue _returnvalue_3))
  (|CallParentFunction)
  (bind _isa (Utilities|FlowControl|FlipFlop)
    (:A
      _)
    (:B
      _))
  (Animation|Montage|PlayMontage (Variables|Character|GetMesh) (select _isa "/Game/AnimAttackRoot_Montage.AnimAttackRoot_Montage" "/Game/AnimAttackRoot1_Montage.AnimAttackRoot1_Montage")
    (:OnNotifyBegin
      (bind (_outhit _returnvalue_5) (Collision|SphereTraceByChannel _returnvalue_4 _returnvalue_4 1e+02 "TraceTypeQuery2" false 0 "ForDuration"))
      (if _returnvalue_5
        (bind _asbp_third_person_character (Utilities|Casting|CastToBP_ThirdPersonCharacter (.HitActor (Collision|BreakHitResult _outhit))))
        (Game|Damage|ApplyDamage _asbp_third_person_character (Variables|Default|GetDamage) 0 0)))))

(fn ConstructionScript
  (|CallParentFunction))