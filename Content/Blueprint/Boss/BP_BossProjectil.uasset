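; Boss projectile that falls through the world and damages the player on contact.
; Tick moves it down by a random per-frame step without sweep or delta-time scaling, while slowly spinning it.
; The first sphere overlap with BP_ThirdPersonCharacter applies damage, prints a debug string, sets the Niagara Curve parameter, then detaches and deactivates the effect.
; A DestroyActor node is left unconnected, so the graph never destroys the actor.
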(event OnComponentBeginOverlap(Sphere1)
  (params (OverlappedComponent :type Primitive%20Component%20Object%20Reference) (OtherActor :type Actor%20Object%20Reference) (OtherComp :type Primitive%20Component%20Object%20Reference) (OtherBodyIndex :type Integer) (bFromSweep :type Boolean) (SweepResult :type Hit%20Result%20Structure%20%28by%20ref%29))
  (bind _niagara (Variables|Default|GetNiagara))
  (bind _asbp_third_person_character (Utilities|Casting|CastToBP_ThirdPersonCharacter OtherActor))
  (Utilities|FlowControl|DoOnce false
    (:Completed
      (Game|Damage|ApplyDamage _asbp_third_person_character 1.0 0 0)
      (Niagara|SetNiagaraVariable(Float) _niagara "Curve" 3e+03)
      (Development|PrintString "Hello")
      (Transformation|DetachFromComponent _niagara "KeepWorld" "KeepWorld" "KeepWorld" true)
      (Components|Activation|Deactivate _niagara))))

(event EventTick
  (params (DeltaSeconds :type Float%20%28single-precision%29))
  (Transformation|AddActorWorldOffset (Math|Vector|MakeVector 0.0 0.0 (* (Math|Random|RandomFloatinRange 4.0 7.0) -1.0)))
  (Transformation|AddActorLocalRotation "0.000000,1.000000,0.000000" false false))

(fn ConstructionScript)