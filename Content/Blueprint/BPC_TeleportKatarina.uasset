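; Actor component that gives the third-person player a Katarina-style bottle teleport on the IA_ThrowBottle input.
; The first press spawns a BP_TeleportBottle at the character's Scene component transform and starts a CDKatarina-length cooldown via Delay.
; The next press teleports the player just above the bottle's current position and destroys it, regardless of the cooldown.
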(event Input|EnhancedActionEvents|EnhancedInputActionIA_ThrowBottle
  (params (ActionValue :type Boolean) (ElapsedSeconds :type Float%20%28double-precision%29) (TriggeredSeconds :type Float%20%28double-precision%29) (InputAction :type Input%20Action%20Object%20Reference :default "/Game/ThirdPerson/Input/Actions/IA_ThrowBottle.IA_ThrowBottle"))
  (bind _scene (Variables|Default|GetScene))
  (:Started
    (if (not (Variables|Default|GetBottlePlaced?))
      (if (Variables|Default|GetCanThrow?)
        (bind _returnvalue (Game|SpawnActorfromClass "/Game/Blueprint/Projectile/BP_TeleportBottle.BP_TeleportBottle_C" (Math|Transform|MakeTransform (Transformation|GetWorldLocation _scene) (Transformation|GetWorldRotation _scene) "1.000000,1.000000,1.000000") "Undefined" "MultiplyWithRoot" 0 0))
        (Variables|Default|SetBottlePlaced? true)
        (Variables|Default|SetCanThrow? false)
        (Utilities|FlowControl|Delay (Variables|Default|GetCDKatarina))
        (Variables|Default|SetCanThrow? true))
      (else
        (Transformation|SetActorLocation (Game|GetPlayerCharacter 0) (+ (Transformation|GetWorldLocation (Variables|/Game/Blueprint/Projectile/BP_TeleportBottle.BP_TeleportBottle_C|GetBottle _returnvalue)) "0.000000,0.000000,125.000000") false true)
        (Variables|Default|SetBottlePlaced? false)
        (Actor|DestroyActor _returnvalue)))))

(event EventBeginPlay
  (bind _asbp_third_person_character (Utilities|Casting|CastToBP_ThirdPersonCharacter (Game|GetPlayerCharacter 0)))
  (Variables|Default|SetScene (Variables|/Game/ThirdPerson/Blueprints/BP_ThirdPersonCharacter.BP_ThirdPersonCharacter_C|GetScene _asbp_third_person_character)))