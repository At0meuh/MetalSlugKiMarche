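; AI controller for enemies that runs the BT_Ennemies behavior tree from BeginPlay and caches the possessed Bp_EnneParent pawn.
; AI perception writes a sensed BP_ThirdPersonCharacter into the Target blackboard key and clears the key when sensing is lost.
; Tick polls the cached pawn's Dead flag and deactivates the Blackboard component while it is set.
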(event OnTargetPerceptionUpdated(AIPerception)
  (params (Actor :type Actor%20Object%20Reference) (Stimulus :type AI%20Stimulus%20Structure))
  (bind _asbp_third_person_character (Utilities|Casting|CastToBP_ThirdPersonCharacter Actor))
  (if (.bSuccessfullySensed (Utilities|Struct|BreakAIStimulus Stimulus))
    (AI|Components|Blackboard|SetValueasObject (Variables|Default|GetBlackboard) (Utilities|Name|MakeLiteralName "Target") _asbp_third_person_character)
    (else
      (AI|Components|Blackboard|SetValueasObject (Variables|Default|GetBlackboard) (Utilities|Name|MakeLiteralName "Target") 0))))

(event EventBeginPlay
  (AI|RunBehaviorTree "/Game/Blueprint/Ennemies/BT_Ennemies.BT_Ennemies"))

(event EventTick
  (params (DeltaSeconds :type Float%20%28single-precision%29))
  (bind _as_bp_enne_parent (Variables|Default|GetAs%20Bp%20Enne%20Parent)
    (:then
      (if (Variables|/Game/Blueprint/Ennemies/Bp_EnneParent.Bp_EnneParent_C|GetDead? _as_bp_enne_parent)
        (Components|Activation|Deactivate (Variables|Default|GetBlackboard))))
    (:else)))

(event EventPossess
  (params (PossessedPawn :type Pawn%20Object%20Reference))
  (bind _asbp_enne_parent (Utilities|Casting|CastToBp_EnneParent PossessedPawn))
  (Variables|Default|SetAs%20Bp%20Enne%20Parent _asbp_enne_parent))

(fn ConstructionScript)