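; Custom game instance that keeps a persistent score record across sessions through a global save slot.
; On Init it loads the existing Bp_Save and copies its Score into the instance, or creates a new save object when none exists.
; The Sauvegarde event appends a new score to the saved Score collection and writes it back to the slot.
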(event Custom|Sauvegarde
  (params (ScoreToAdd :type ST%20Score%20Structure))
  (bind _as_bp_save (Variables|Default|GetAs%20Bp%20Save))
  (Utilities|Array|Add (Variables|/Game/Blueprint/Bp_Save.Bp_Save_C|GetScore _as_bp_save) ScoreToAdd)
  (SaveGame|SaveGametoSlot _as_bp_save "SaveGlobal"))

(event EventInit
  (bind _returnvalue (SaveGame|DoesSaveGameExist "SaveGlobal"))
  (if _returnvalue
    (bind _returnvalue_2 (SaveGame|LoadGamefromSlot "SaveGlobal"))
    (bind _asbp_save (Utilities|Casting|CastToBp_Save _returnvalue_2))
    (bind _output_get (Variables|Default|SetAs%20Bp%20Save _asbp_save))
    (Variables|Default|SetScore (Variables|/Game/Blueprint/Bp_Save.Bp_Save_C|GetScore _output_get))
    (else
      (bind _returnvalue_3 (SaveGame|CreateSaveGameObject "/Game/Blueprint/Bp_Save.Bp_Save_C"))
      (Variables|Default|SetAs%20Bp%20Save _returnvalue_3))))