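; Flamethrower weapon that the third-person character auto-equips on overlapping its box, spraying Niagara fire that damages nearby enemies.
; Fire and EndFire toggle the effect, ammo drain and Wwise sound, while Tick feeds player velocity to Niagara and plays force feedback.
; A capsule tracks actors implementing BPI_FlammeThrower, and ParticleData damages them all, with the weapon registered as the Niagara system's Target object.
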(event OnComponentBeginOverlap(Box)
  (params (OverlappedComponent :type Primitive%20Component%20Object%20Reference) (OtherActor :type Actor%20Object%20Reference) (OtherComp :type Primitive%20Component%20Object%20Reference) (OtherBodyIndex :type Integer) (bFromSweep :type Boolean) (SweepResult :type Hit%20Result%20Structure%20%28by%20ref%29))
  (bind _asbp_third_person_character (Utilities|Casting|CastToBP_ThirdPersonCharacter OtherActor))
  (Variables|Default|SetAs%20BP%20Third%20Person%20Character _asbp_third_person_character)
  (Utilities|Array|AddUnique (Variables|/Game/ThirdPerson/Blueprints/BP_ThirdPersonCharacter.BP_ThirdPersonCharacter_C|GetWeaponsTab _asbp_third_person_character) self)
  (Default|EquipWeapon _asbp_third_person_character self)
  (Class|NiagaraComponent|SetVariableObject (Variables|Default|GetNiagara) "Target" self))

(event OnComponentBeginOverlap(EnnemiesTriggerZone)
  (params (OverlappedComponent :type Primitive%20Component%20Object%20Reference) (OtherActor :type Actor%20Object%20Reference) (OtherComp :type Primitive%20Component%20Object%20Reference) (OtherBodyIndex :type Integer) (bFromSweep :type Boolean) (SweepResult :type Hit%20Result%20Structure%20%28by%20ref%29)))

(event OnComponentEndOverlap(EnnemiesTriggerZone)
  (params (OverlappedComponent :type Primitive%20Component%20Object%20Reference) (OtherActor :type Actor%20Object%20Reference) (OtherComp :type Primitive%20Component%20Object%20Reference) (OtherBodyIndex :type Integer)))

(event OnComponentBeginOverlap(Capsule)
  (params (OverlappedComponent :type Primitive%20Component%20Object%20Reference) (OtherActor :type Actor%20Object%20Reference) (OtherComp :type Primitive%20Component%20Object%20Reference) (OtherBodyIndex :type Integer) (bFromSweep :type Boolean) (SweepResult :type Hit%20Result%20Structure%20%28by%20ref%29))
  (if (Utilities|DoesObjectImplementInterface OtherActor "/Game/Blueprint/weapon/BPI_FlammeThrower.BPI_FlammeThrower_C")
    (Utilities|Array|AddUnique (Variables|Default|GetEnnemiesInRanged) OtherActor)))

(event OnComponentEndOverlap(Capsule)
  (params (OverlappedComponent :type Primitive%20Component%20Object%20Reference) (OtherActor :type Actor%20Object%20Reference) (OtherComp :type Primitive%20Component%20Object%20Reference) (OtherBodyIndex :type Integer))
  (Utilities|Array|RemoveItem (Variables|Default|GetEnnemiesInRanged) OtherActor))

(event EventTick
  (params (DeltaSeconds :type Float%20%28single-precision%29))
  (bind _niagara (Variables|Default|GetNiagara))
  (bind _as_bp_third_person_character (Variables|Default|GetAs%20BP%20Third%20Person%20Character)
    (:then
      (Class|NiagaraComponent|SetNiagaraVariableVec3 _niagara "PlayerVelocity" (* (Transformation|GetVelocity _as_bp_third_person_character) (Math|Float|NormalizetoRange (Class|NiagaraComponent|GetDesiredAge _niagara) 1.0 1.5)))
      (if (Variables|Default|Get--Ammo)
        (bind _output_get (Variables|Default|SetAmmo++ (- (Variables|Default|GetAmmo++) (Utilities|Time|GetWorldDeltaSeconds))))
        (Game|Feedback|ClientPlayForceFeedback (Game|GetPlayerController 0) "/Game/FF_FlameThrower.FF_FlameThrower" "None" false false false)
        (Variables|Default|SetAmmo (Math|Float|Truncate (Variables|Default|GetAmmo++)))
        (if (<= _output_get 0.0)
          (CallFunction|EndFire))))
    (:else)))

(event EventParticleData
  (params (Data :type Array%20of%20Basic%20Particle%20Data%20Structures) (NiagaraSystem :type Niagara%20System%20Object%20Reference) (SimulationPositionOffset :type Vector%20%28by%20ref%29 :default "0, 0, 0"))
  (for _array_element (Variables|Default|GetEnnemiesInRanged)
    (Game|Damage|ApplyDamage _array_element (Variables|Default|GetFireDamage) 0 0)))

(event EventEndFire
  ;[0.01096 0.01161 0.0137] Collision feu niagara
  (Components|Activation|Deactivate (Variables|Default|GetNiagara))
  (Utilities|Time|ClearandInvalidateTimerbyHandle (Variables|Default|GetFireTrace))
  (Variables|Default|Set--Ammo false)
  (Class|AkGameplayStatics|PostEvent "/Game/WwiseAudio/Event/Stop_SFX_Flamewother.Stop_SFX_Flamewother")
  (Utilities|FlowControl|DoOnce false) ; enters at Reset
)

(event EventFire
  ;[0.01096 0.01161 0.0137] Collision feu niagara
  (Utilities|FlowControl|Sequence
    (:then_0
      (Components|Activation|Activate (Variables|Default|GetNiagara) true)
      (Variables|Default|Set--Ammo true))
    (:then_1
      (Utilities|FlowControl|DoOnce false
        (:Completed
          (Class|AkGameplayStatics|PostEvent "/Game/WwiseAudio/Event/Play_SFX_Flamewother.Play_SFX_Flamewother"))))))

(event EventBeginPlay
  (Variables|Default|SetAmmo++ (Math|Conversions|ToFloat(Integer) (Variables|Default|GetAmmo))))

(fn ConstructionScript
  (|CallParentFunction)
  (Transformation|SetRelativeLocation (Variables|Default|GetNiagara) (Variables|/Script/Engine.SceneComponent|GetRelativeLocation (Variables|Default|GetProjectileSpawn)) false false))