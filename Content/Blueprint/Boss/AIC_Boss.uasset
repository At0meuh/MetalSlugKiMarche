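; AI controller for the boss that runs the BT_Boss behavior tree on BeginPlay.
; On possess it caches the BP_Boss pawn, then polls it each Tick and deactivates the Blackboard once the boss is dead.
; StartPatern sets the Blackboard's Start bool and prints a debug string.
; An unconnected node that would set Target to the player controller never runs.
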(event Custom|StartPatern
  (params (BoolValue :type Boolean))
  (Development|PrintString "Hello")
  (AI|Components|Blackboard|SetValueasBool (Variables|Default|GetBlackboard) (Utilities|Name|MakeLiteralName "Start") BoolValue))

(event EventBeginPlay
  (AI|RunBehaviorTree "/Game/Blueprint/Boss/BT_Boss.BT_Boss"))

(event EventTick
  (params (DeltaSeconds :type Float%20%28single-precision%29))
  (bind _as_bp_boss (Variables|Default|GetAs%20BP%20Boss)
    (:then
      (if (Variables|/Game/Blueprint/Boss/BP_Boss.BP_Boss_C|GetDead? _as_bp_boss)
        (Components|Activation|Deactivate (Variables|Default|GetBlackboard))))
    (:else)))

(event EventPossess
  (params (PossessedPawn :type Pawn%20Object%20Reference))
  (bind _asbp_boss (Utilities|Casting|CastToBP_Boss PossessedPawn))
  (Variables|Default|SetAs%20BP%20Boss _asbp_boss))

(fn ConstructionScript)